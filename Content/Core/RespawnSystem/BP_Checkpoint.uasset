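; BP_Checkpoint is a checkpoint actor that moves the respawn point when its trigger box is overlapped.
; Any overlap sends the Arrow component's world transform and a self reference to GM_MyProject3D through UpdateRespawnPoint, then swaps the button mesh to its alternate material.
; A ReturnToNormal event restores the default button material, with no caller inside this Blueprint.
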(event `self.Box.OnComponentBeginOverlap`
  (params (OverlappedComponent :type "PrimitiveComponent Object Reference") (OtherActor :type "Actor Object Reference") (OtherComp :type "PrimitiveComponent Object Reference") (OtherBodyIndex :type Integer) (bFromSweep :type Boolean) (SweepResult :type "HitResult Structure (by ref)"))
  (bind _asgm_my_project_3d (cast `/Game/Core/Framework/GM_MyProject3D` (`GameplayStatics.GetGameMode`)))
  (`/Game/Core/Framework/GM_MyProject3D.UpdateRespawnPoint` _asgm_my_project_3d (`SceneComponent.K2_GetComponentToWorld` (`self.Arrow`)) self)
  (`PrimitiveComponent.SetMaterial` (`self.SM Button A Push`) 0 "/Game/TeachersMarketplace/Assets/Props/Buttons/Button_A/Material/M_Button_A_2.M_Button_A_2"))

(event `ReturnToNormal`
  (`PrimitiveComponent.SetMaterial` (`self.SM Button A Push`) 0 "/Game/TeachersMarketplace/Assets/Props/Buttons/Button_A/Material/M_Button_A.M_Button_A"))

(fn `UserConstructionScript`)