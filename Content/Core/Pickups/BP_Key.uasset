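; BP_Key is a key pickup that grants the main character a key when collected.
; It overrides the PickedThisUp event, calls the parent implementation, then casts the picker to BP_MainCharacter and calls GetAKey with its KeyType.
; BeginPlay, overlap and Tick are disabled stubs, and the construction script only calls the parent.
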(event `self.PickedThisUp`
  (params (ActorThePickedUpThis :type "Actor Object Reference"))
  (`parent.PickedThisUp` ActorThePickedUpThis)
  (bind _asbp_main_character (cast `/Game/Core/Player/BP_MainCharacter` ActorThePickedUpThis))
  (`/Game/Core/Player/BP_MainCharacter.GetAKey` _asbp_main_character (`self.KeyType`)))

(fn `UserConstructionScript`
  (`parent.UserConstructionScript`))