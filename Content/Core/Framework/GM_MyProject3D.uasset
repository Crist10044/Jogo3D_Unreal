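; Game mode that tracks the player's respawn point and handles winning the game.
; BeginPlay seeds the respawn transform from a PlayerStart found in the level.
; UpdateRespawnPoint reverts the stored checkpoint to normal and saves the new transform, but reassigns the checkpoint variable to itself, leaving the CheckpointRef input unused.
; WinTheGame prints a Portuguese victory message and puts BP_MainCharacter into celebration.
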(event `self.ReceiveBeginPlay`
  (bind _returnvalue (`GameplayStatics.GetActorOfClass` "/Script/Engine.PlayerStart"))
  (set `self.RespawnPoint` (`self.GetTransform` _returnvalue)))

(event `WinTheGame`
  (`KismetSystemLibrary.PrintString` "VOCÊ VENCEU! :D")
  (bind _asbp_main_character (cast `/Game/Core/Player/BP_MainCharacter` (`GameplayStatics.GetPlayerCharacter` 0)))
  (`/Game/Core/Player/BP_MainCharacter.EnterCelebration` _asbp_main_character))

(fn `UpdateRespawnPoint`
  (params (NewRespawnPoint :type "Transform Structure") (CheckpointRef :type "Object Object Reference"))
  (bind _currentcheckpoint_ref (`self.CurrentCheckpoint Ref`))
  (`|ExecutionSequence`
    (:`then_0`
      (if (`KismetSystemLibrary.IsValid` _currentcheckpoint_ref)
        (`/Game/Core/RespawnSystem/BP_Checkpoint.ReturnToNormal` _currentcheckpoint_ref)))
    (:`then_1`
      (set `self.RespawnPoint` (`local.NewRespawnPoint`))
      (set `self.CurrentCheckpoint Ref` (`self.CurrentCheckpoint Ref`)))))

(fn `UserConstructionScript`)